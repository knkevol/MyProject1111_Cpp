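; BP_GM holds the stage-clear rule that moves the game on to the next level.
; Its custom Rule event finds all actors tagged Target and, when none remain, prints a clear message.
; After a short delay it reads NextStage from the first BP_Stage actor and opens that level by name, so each stage defines its own successor.
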(event Custom|Rule
  (bind _outactors (Actor|GetAllActorswithTag "Target"))
  (if (== (Utilities|Array|Length _outactors) 0)
    (Development|PrintString "Clear!")
    (Utilities|FlowControl|Delay 2.0)
    (bind _outactors_2 (Actor|GetAllActorsOfClass "/Game/Blueprints/BP_Stage.BP_Stage_C"))
    (Game|OpenLevel(byName) (Utilities|String|StringToName (Variables|/Game/Blueprints/BP_Stage.BP_Stage_C|GetNextStage (Utilities|Array|Get(acopy) _outactors_2))))))

(fn ConstructionScript)